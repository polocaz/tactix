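; BP_Enemy is a damageable enemy that attacks on a looping timer and ragdolls when it dies.
; Each attack sphere-traces forward for pawns with debug drawing, sends a damage message to the hit actor and spawns an explosion if it succeeds.
; Health, healing and damage calls forward to BPHealthComponent, whose death, block and damage-response events are bound in the construction script.
; A widget component shows its health bar.
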(event `self.ReceiveBeginPlay`
  (`|ExecutionSequence`
    (:`then_0`
      (bind _returnvalue (`|CreateWidget` "/Game/DamageSystem/W_HealthBar.W_HealthBar_C" null self))
      (`WidgetComponent.SetWidget` (`self.HealthBar`) _returnvalue))
    (:`then_1`
      (`KismetSystemLibrary.K2_SetTimerDelegate` (delegate `Attack`) 2.0 true))))

(event `Attack`
  (bind _returnvalue (`KismetMathLibrary.MakeVector` (.x (`self.K2_GetActorLocation`)) (.y (`self.K2_GetActorLocation`)) (+ (.z (`self.K2_GetActorLocation`)) 60.0)))
  (if (not (`/Game/DamageSystem/BP_HealthComponent.IsDead` (`self.BP_HealthComponent`)))
    (bind (_outhit _returnvalue_2) (`KismetSystemLibrary.SphereTraceSingleForObjects` :`Start` _returnvalue :`End` (+ _returnvalue (* (`self.GetActorForwardVector`) 100.0)) :`Radius` 20.0 :`ObjectTypes` (`|MakeArray` "ObjectTypeQuery3" :!type "EObjectTypeQuery Enum") :`DrawDebugType` "ForDuration" :`TraceColor` (struct :`R` 1.0 :`G` 0.021001 :`B` 0.75086 :`A` 1.0) :`TraceHitColor` (struct :`G` 0.045198 :`B` 1.0 :`A` 1.0) :`DrawTime` 1.0))
    (if _returnvalue_2
      (bind (_bblockinghit _binitialoverlap _time _distance _location _impactpoint _normal _impactnormal _physmat _hitactor) (`GameplayStatics.BreakHitResult` _outhit))
      (bind _wasdamaged (message `/Game/DamageSystem/BPI_Damageable.TakeDamage` _hitactor (make `/Game/DamageSystem/S_DamageInfo` 50.0 "NewEnumerator4" "NewEnumerator6")))
      (if _wasdamaged
        (`GameplayStatics.SpawnEmitterAtLocation` "/Game/StarterContent/Particles/P_Explosion.P_Explosion" _impactpoint)))))

(event `StartDeath`
  (bind _mesh (`self.Mesh`))
  (`PrimitiveComponent.SetSimulatePhysics` _mesh true)
  (`PrimitiveComponent.SetCollisionEnabled` _mesh "QueryAndPhysics")
  (`PrimitiveComponent.SetCollisionEnabled` (`self.CapsuleComponent`) "NoCollision")
  (`SkeletalMeshComponent.Stop` (`self.Mesh`)))

(event `StartBlock`
  (params (CanBeParried :type Boolean))
  (`KismetSystemLibrary.PrintString` "BLOCKED"))

(event `RespondToDamage`
  (params (DamageResponse :type "EDamageResponse Enum" :default "None"))
  (`KismetSystemLibrary.PrintString` (`|GetEnumeratorNameAsString` DamageResponse)))

(fn `GetCurrentHealth`
  (returns (CurrentHealth :type "Float (double-precision)"))
  (return (`/Game/DamageSystem/BP_HealthComponent.Health` (`self.BP_HealthComponent`))))

(fn `GetMaxHealth`
  (returns (MaxHealth :type "Float (double-precision)"))
  (return (`/Game/DamageSystem/BP_HealthComponent.MaxHealth` (`self.BP_HealthComponent`))))

(fn `PerformHeal`
  (params (HealAmount :type "Float (double-precision)"))
  (returns (NewHealth :type "Float (double-precision)"))
  (bind _newhealth (`/Game/DamageSystem/BP_HealthComponent.AddHealth` (`self.BP_HealthComponent`) HealAmount))
  (return _newhealth))

(fn `ReceiveDamage`
  (params (DamageInfo :type "DamageInfo Structure"))
  (returns (WasDamaged :type Boolean))
  (bind _wasdamaged (`/Game/DamageSystem/BP_HealthComponent.ReceiveDamage` (`self.BP_HealthComponent`) DamageInfo))
  (return _wasdamaged))

(fn `UserConstructionScript`
  (bind _bp_healthcomponent (`self.BP_HealthComponent`))
  (add `/Game/DamageSystem/BP_HealthComponent.OnDeath` _bp_healthcomponent (`|CreateDelegate` :!event `StartDeath`))
  (add `/Game/DamageSystem/BP_HealthComponent.OnBlocked` _bp_healthcomponent (`|CreateDelegate` :!event `StartBlock`))
  (add `/Game/DamageSystem/BP_HealthComponent.OnDamageResponse` _bp_healthcomponent (`|CreateDelegate` :!event `RespondToDamage`)))