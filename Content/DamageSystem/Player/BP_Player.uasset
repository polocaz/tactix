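; Player character for a damage system, with a health bar widget and a BPHealthComponent that backs healing and health queries.
; Construction script binds the component's death, blocked and damage-response events; death ragdolls the mesh and disables input, while the others print debug text.
; Left click runs a debug sphere-trace attack that sends damage by message, and a debug key heals.
; Several damage and health functions, including TakeDamage and ReceiveDamage, are empty stubs.
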(event Custom|StartDeath
  (bind _mesh (Variables|Character|GetMesh))
  (Physics|SetSimulatePhysics _mesh true)
  (Collision|SetCollisionEnabled _mesh "QueryAndPhysics")
  (Collision|SetCollisionEnabled (Variables|Default|GetCapsuleComponent) "NoCollision")
  (Input|DisableInput (Game|GetPlayerController 0)))

(event Custom|StartBlock
  (params (CanBeParried :type Boolean))
  (Development|PrintString "BLOCKED"))

(event Custom|RespondToDamage
  (params (DamageResponse :type E_DamageResponse%20Enum :default "NewEnumerator5"))
  (Development|PrintString (Utilities|String|EnumtoString DamageResponse)))

(event EventBeginPlay
  (bind _returnvalue (UserInterface|CreateWidget "/Game/DamageSystem/W_HealthBar.W_HealthBar_C" 0 self))
  (UserInterface|SetWidget (Variables|Default|GetHealth) _returnvalue))

(event Input|KeyboardEvents|DebugKeyH
  (params (Key :type Key%20Structure) (ActionValue :type Input%20Action%20Value%20Structure))
  (:Pressed
    (CallFunction|PerformHealBP 2e+01)))

(event Input|MouseEvents|LeftMouseButton
  (params (Key :type Key%20Structure))
  (:Pressed
    (CallFunction|DebugAttack)))

(fn ConstructionScript
  (bind _bp_healthcomponent (Variables|Default|GetBP_HealthComponent))
  (EventDispatchers|BindEventtoOnDeath _bp_healthcomponent (EventDispatchers|CreateEvent :!event Custom|StartDeath))
  (EventDispatchers|BindEventtoOnBlocked _bp_healthcomponent (EventDispatchers|CreateEvent :!event Custom|StartBlock))
  (EventDispatchers|BindEventtoOnDamageResponse _bp_healthcomponent (EventDispatchers|CreateEvent :!event Custom|RespondToDamage)))

(fn DebugAttack
  (bind _returnvalue (Transformation|GetActorLocation))
  (bind (_x _y _z) (Math|Vector|BreakVector _returnvalue))
  (bind _returnvalue_2 (+ _z 6e+01))
  (bind _returnvalue_3 (Math|Vector|MakeVector _x _y _returnvalue_2))
  (bind (_outhit _returnvalue_4) (Collision|SphereTraceForObjects _returnvalue_3 (+ _returnvalue_3 (* (Math|Vector|GetForwardVector (Variables|Default|GetFollowCamera)) 1e+02)) 2e+01 (Utilities|Array|MakeArray "ObjectTypeQuery3") false 0 "ForDuration" true "(R=1.000000,G=0.000000,B=0.000000,A=1.000000)" "(R=0.000000,G=1.000000,B=0.000000,A=1.000000)" 1.0))
  (if _returnvalue_4
    (bind _wasdamaged (Class|BPIDamageable|TakeDamage(Message) (.HitActor (Collision|BreakHitResult _outhit)) (Utilities|Struct|MakeS_DamageInfo 5e+01 "NewEnumerator4" "NewEnumerator6")))
    (if _wasdamaged
      (Effects|SpawnEmitteratLocation "/Game/StarterContent/Particles/P_Explosion.P_Explosion" (.ImpactPoint (Collision|BreakHitResult _outhit))))))

(fn TakeDamageBP
  (return))

(fn TakeDamage
  (params (DamageInfo :type S%20Damage%20Info%20Structure))
  (return false))

(fn PerformHealBP
  (params (HealAmount :type Float%20%28double-precision%29))
  (bind _newhealth (Default|AddHealth (Variables|Default|GetBP_HealthComponent) HealAmount))
  (return _newhealth))

(fn GetMaxHealthBP
  (return (Variables|/Game/DamageSystem/BP_HealthComponent.BP_HealthComponent_C|GetMaxHealth (Variables|Default|GetBP_HealthComponent))))

(fn GetCurrentHealthBP
  (return (Variables|/Game/DamageSystem/BP_HealthComponent.BP_HealthComponent_C|GetHealth (Variables|Default|GetBP_HealthComponent))))

(fn GetCurrentHealth
  (return 0.0))

(fn GetMaxHealth
  (return 0.0))

(fn PerformHeal
  (params (HealAmount :type Float%20%28double-precision%29))
  (return 0.0))

(fn ReceiveDamage
  (params (DamageInfo :type Damage%20Info%20Structure))
  (return false))