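; Health component that tracks an actor's health, healing and death, and resolves incoming damage described by a DamageInfo struct.
; A CanBeDamaged macro routes each hit to block, damage or no damage using dead, invincible and blocking states.
; TakeDamage and ReceiveDamage share identical logic, firing OnBlocked, OnDeath, or OnDamageResponse when the hit can interrupt.
; AddHealth heals the living within the health limits.
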(fn `AddHealth`
  (params (Amount :type "Float (double-precision)"))
  (returns (NewHealth :type "Float (double-precision)"))
  (if (not (`self.IsDead`))
    (bind _output_get (set `self.Health` (`KismetMathLibrary.FClamp` (+ Amount (`self.Health`)) 0.0 (`self.MaxHealth`))))
    (return _output_get)))

(fn `ReceiveDamage`
  (params (DamageInfo :type "DamageInfo Structure"))
  (returns (WasDamaged :type Boolean))
  (bind (_damageamount _damagetype _damageresponse _bshoulddamageinvincible _bcanbeblocked _bcanbeparried _bshouldforceinterrupt) (break `DamageInfo` DamageInfo))
  (`self.CanBeDamaged` _bshoulddamageinvincible _bcanbeblocked
    (:`BlockDamage`
      (`self.OnBlocked` _bcanbeparried)
      (return false))
    (:`DoDamage`
      (bind _output_get (set `self.Health` (- (`self.Health`) _damageamount)))
      (if (<= _output_get 0.0)
        (set `self.IsDead` true)
        (`self.OnDeath`)
        (return true)
        (elif (or (`self.IsInterruptible`) _bshouldforceinterrupt)
          (`self.OnDamageResponse` _damageresponse)
          (return true))))
    (:`NoDamage`
      (return false))))

(fn `TakeDamage`
  (params (DamageInfo :type "DamageInfo Structure"))
  (returns (WasDamaged :type Boolean))
  (bind (_damageamount _damagetype _damageresponse _bshoulddamageinvincible _bcanbeblocked _bcanbeparried _bshouldforceinterrupt) (break `DamageInfo` DamageInfo))
  (`self.CanBeDamaged` _bshoulddamageinvincible _bcanbeblocked
    (:`BlockDamage`
      (`self.OnBlocked` _bcanbeparried)
      (return false))
    (:`DoDamage`
      (bind _output_get (set `self.Health` (- (`self.Health`) _damageamount)))
      (if (<= _output_get 0.0)
        (set `self.IsDead` true)
        (`self.OnDeath`)
        (return true)
        (elif (or (`self.IsInterruptible`) _bshouldforceinterrupt)
          (`self.OnDamageResponse` _damageresponse)
          (return true))))
    (:`NoDamage`
      (return false))))