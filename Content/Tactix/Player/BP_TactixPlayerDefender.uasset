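; Player defender character Blueprint for Tactix that gives the player a demo pistol and handles combat input.
; On BeginPlay it equips BP_DemoPistol through its Tactix weapon component.
; Enhanced Input attack press and release start and stop attacking, and reload triggers a reload, all forwarded to that component after validity checks.
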(event `self.ReceiveBeginPlay`
  (bind _bp_tactixweaponcomponent (`self.BP_TactixWeaponComponent`))
  (`parent.ReceiveBeginPlay`)
  (`WeaponComponent.EquipWeaponByClass` _bp_tactixweaponcomponent "/Game/Tactix/Weapons/Guns/BP_DemoPistol.BP_DemoPistol_C")
  (`/Engine/EditorBlueprintResources/StandardMacros.IsValid` (`WeaponComponent.CurrentWeapon` _bp_tactixweaponcomponent)))

(event `EnhancedInput|/Game/Tactix/Input/Actions/IA_Attack`
  (params (ActionValue :type Boolean) (ElapsedSeconds :type "Float (double-precision)") (TriggeredSeconds :type "Float (double-precision)") (InputAction :type "InputAction Object Reference" :default "/Game/Tactix/Input/Actions/IA_Attack.IA_Attack"))
  (bind _bp_tactixweaponcomponent (`self.BP_TactixWeaponComponent`))
  (:`Started`
    (`/Engine/EditorBlueprintResources/StandardMacros.IsValid` _bp_tactixweaponcomponent
      (:`Is Valid`
        (`/Engine/EditorBlueprintResources/StandardMacros.IsValid` (`WeaponComponent.CurrentWeapon` _bp_tactixweaponcomponent)
          (:`Is Valid`
            (`WeaponComponent.StartAttack` _bp_tactixweaponcomponent))))))
  (:`Completed`
    (`/Engine/EditorBlueprintResources/StandardMacros.IsValid` _bp_tactixweaponcomponent
      (:`Is Valid`
        (`WeaponComponent.StopAttack` _bp_tactixweaponcomponent)))))

(event `EnhancedInput|/Game/Tactix/Input/Actions/IA_Reload`
  (params (ActionValue :type Boolean) (ElapsedSeconds :type "Float (double-precision)") (TriggeredSeconds :type "Float (double-precision)") (InputAction :type "InputAction Object Reference" :default "/Game/Tactix/Input/Actions/IA_Reload.IA_Reload"))
  (bind _bp_tactixweaponcomponent (`self.BP_TactixWeaponComponent`))
  (:`Started`
    (`/Engine/EditorBlueprintResources/StandardMacros.IsValid` _bp_tactixweaponcomponent
      (:`Is Valid`
        (`/Engine/EditorBlueprintResources/StandardMacros.IsValid` (`WeaponComponent.CurrentWeapon` _bp_tactixweaponcomponent)
          (:`Is Valid`
            (`WeaponComponent.Reload` _bp_tactixweaponcomponent)))))))

(fn `UserConstructionScript`
  (`parent.UserConstructionScript`))