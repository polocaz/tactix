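; BP_TactixPlayerBase is a base player Blueprint for Tactix that exposes health queries, healing and damage handling.
; Its four health functions are thin wrappers that read from or forward to BPHealthComponent, returning that component's results.
; The event graph does nothing at runtime: Possessed is empty, and logic adding the IMC_MouseLook Enhanced Input mapping context for player controllers is left unconnected.
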(event `self.ReceivePossessed`
  (params (NewController :type "Controller Object Reference")))

(fn `GetCurrentHealth`
  (returns (CurrentHealth :type "Float (double-precision)"))
  (return (`/Game/DamageSystem/BP_HealthComponent.Health` (`self.BP_HealthComponent`))))

(fn `GetMaxHealth`
  (returns (MaxHealth :type "Float (double-precision)"))
  (return (`/Game/DamageSystem/BP_HealthComponent.MaxHealth` (`self.BP_HealthComponent`))))

(fn `PerformHeal`
  (params (HealAmount :type "Float (double-precision)"))
  (returns (NewHealth :type "Float (double-precision)"))
  (bind _newhealth (`/Game/DamageSystem/BP_HealthComponent.AddHealth` (`self.BP_HealthComponent`) HealAmount))
  (return _newhealth))

(fn `ReceiveDamage`
  (params (DamageInfo :type "DamageInfo Structure"))
  (returns (WasDamaged :type Boolean))
  (bind _wasdamaged (`/Game/DamageSystem/BP_HealthComponent.ReceiveDamage` (`self.BP_HealthComponent`) DamageInfo))
  (return _wasdamaged))

(fn `UserConstructionScript`)