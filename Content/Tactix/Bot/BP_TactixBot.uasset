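; BP_TactixBot is an armed character with health that equips a demo pistol at BeginPlay and shows a crosshair on the player screen.
; Enhanced Input attack and reload actions drive the weapon component.
; The health component handles damage, healing and health queries through wrapper functions, with its OnDeath event bound in the construction script.
; StartDeath ragdolls the mesh and disables capsule collision.
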(event `self.ReceiveBeginPlay`
  (bind _bp_tactixweaponcomponent (`self.BP_TactixWeaponComponent`))
  (`parent.ReceiveBeginPlay`)
  (`WeaponComponent.EquipWeaponByClass` _bp_tactixweaponcomponent "/Game/Tactix/Weapons/Guns/BP_DemoPistol.BP_DemoPistol_C")
  (`/Engine/EditorBlueprintResources/StandardMacros.IsValid` (`WeaponComponent.CurrentWeapon` _bp_tactixweaponcomponent)
    (:`Is Valid`
      (bind _returnvalue (`|CreateWidget` "/Game/Tactix/UI/WB_Crosshair.WB_Crosshair_C"))
      (`UserWidget.AddToPlayerScreen` _returnvalue 0))))

(event `EnhancedInput|/Game/Tactix/Input/Actions/IA_Attack`
  (params (ActionValue :type Boolean) (ElapsedSeconds :type "Float (double-precision)") (TriggeredSeconds :type "Float (double-precision)") (InputAction :type "InputAction Object Reference" :default "/Game/Tactix/Input/Actions/IA_Attack.IA_Attack"))
  (bind _bp_tactixweaponcomponent (`self.BP_TactixWeaponComponent`))
  (:`Started`
    (`/Engine/EditorBlueprintResources/StandardMacros.IsValid` _bp_tactixweaponcomponent
      (:`Is Valid`
        (`/Engine/EditorBlueprintResources/StandardMacros.IsValid` (`WeaponComponent.CurrentWeapon` _bp_tactixweaponcomponent)
          (:`Is Valid`
            (`WeaponComponent.StartAttack` _bp_tactixweaponcomponent))))))
  (:`Completed`
    (`/Engine/EditorBlueprintResources/StandardMacros.IsValid` _bp_tactixweaponcomponent
      (:`Is Valid`
        (`WeaponComponent.StopAttack` _bp_tactixweaponcomponent)))))

(event `EnhancedInput|/Game/Tactix/Input/Actions/IA_Reload`
  (params (ActionValue :type Boolean) (ElapsedSeconds :type "Float (double-precision)") (TriggeredSeconds :type "Float (double-precision)") (InputAction :type "InputAction Object Reference" :default "/Game/Tactix/Input/Actions/IA_Reload.IA_Reload"))
  (bind _bp_tactixweaponcomponent (`self.BP_TactixWeaponComponent`))
  (:`Started`
    (`/Engine/EditorBlueprintResources/StandardMacros.IsValid` _bp_tactixweaponcomponent
      (:`Is Valid`
        (`/Engine/EditorBlueprintResources/StandardMacros.IsValid` (`WeaponComponent.CurrentWeapon` _bp_tactixweaponcomponent)
          (:`Is Valid`
            (`WeaponComponent.Reload` _bp_tactixweaponcomponent)))))))

(event `Start Death`
  (bind _mesh (`self.Mesh`))
  (`PrimitiveComponent.SetSimulatePhysics` _mesh true)
  (`PrimitiveComponent.SetCollisionEnabled` _mesh "QueryAndPhysics")
  (`PrimitiveComponent.SetCollisionEnabled` (`self.CapsuleComponent`) "NoCollision")
  (`SkeletalMeshComponent.Stop` (`self.Mesh`)))

(fn `GetCurrentHealth`
  (returns (CurrentHealth :type "Float (double-precision)"))
  (return (`/Game/DamageSystem/BP_HealthComponent.Health` (`self.BP_HealthComponent`))))

(fn `GetMaxHealth`
  (returns (MaxHealth :type "Float (double-precision)"))
  (return (`/Game/DamageSystem/BP_HealthComponent.MaxHealth` (`self.BP_HealthComponent`))))

(fn `PerformHeal`
  (params (HealAmount :type "Float (double-precision)"))
  (returns (NewHealth :type "Float (double-precision)"))
  (bind _newhealth (`/Game/DamageSystem/BP_HealthComponent.AddHealth` (`self.BP_HealthComponent`) HealAmount))
  (return _newhealth))

(fn `ReceiveDamage`
  (params (DamageInfo :type "DamageInfo Structure"))
  (returns (WasDamaged :type Boolean))
  (bind _wasdamaged (`/Game/DamageSystem/BP_HealthComponent.ReceiveDamage` (`self.BP_HealthComponent`) DamageInfo))
  (return _wasdamaged))

(fn `UserConstructionScript`
  (`parent.UserConstructionScript`)
  (add `/Game/DamageSystem/BP_HealthComponent.OnDeath` (`self.BP_HealthComponent`) (`|CreateDelegate` :!event `Start Death`)))